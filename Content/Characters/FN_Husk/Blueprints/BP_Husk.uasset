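; Husk enemy character that chases sensed Fortress pawns, melees them and dies when its health runs out.
; PawnSensing drives AIMoveTo, and a box overlap starts a swipe montage that shrinks the box to zero.
; When the swipe completes, a debug-drawn forward trace damages a hit Fortress pawn and restores the box, allowing overlap to retrigger.
; Death deactivates movement, plays a hit-react montage with smoke, then destroys the actor after a delay.
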(event OnSeePawn(PawnSensing)
  (params (Pawn :type Pawn%20Object%20Reference))
  (bind _asfortress_pawn (Utilities|Casting|CastToFortressPawn Pawn))
  (AI|AIMoveTo self (Transformation|GetActorLocation _asfortress_pawn) _asfortress_pawn 5.0 false))

(event OnComponentBeginOverlap(Box)
  (params (OverlappedComponent :type Primitive%20Component%20Object%20Reference) (OtherActor :type Actor%20Object%20Reference) (OtherComp :type Primitive%20Component%20Object%20Reference) (OtherBodyIndex :type Integer) (bFromSweep :type Boolean) (SweepResult :type Hit%20Result%20Structure%20%28by%20ref%29))
  (Utilities|Casting|CastToFortressPawn OtherActor)
  (CallFunction|Attack))

(event Custom|Attack
  (bind _scene (Variables|Default|GetScene))
  (bind _returnvalue (Transformation|GetWorldLocation _scene))
  (Animation|Montage|PlayMontage (Variables|Character|GetMesh) "/Game/Characters/FN_Husk/Animations/Swipe.Swipe"
    (:then
      (Transformation|SetRelativeScale3D (Variables|Default|GetBox) "0, 0, 0"))
    (:OnCompleted
      (bind (_outhit _returnvalue_2) (Collision|LineTraceByChannel _returnvalue (+ _returnvalue (* (Math|Vector|GetForwardVector (Transformation|GetWorldRotation _scene)) 3e+02)) "TraceTypeQuery1" false 0 "ForDuration"))
      (if _returnvalue_2
        (bind _asfortress_pawn (Utilities|Casting|CastToFortressPawn (.HitActor (Collision|BreakHitResult _outhit))))
        (Game|Damage|ApplyDamage _asfortress_pawn 2e+01 0 self)
        (Transformation|SetRelativeScale3D (Variables|Default|GetBox) "1.000000,1.000000,2.250000")))))

(event EventBeginPlay)

(event Game|Damage|EventAnyDamage
  (params (Damage :type Float%20%28single-precision%29) (DamageType :type Damage%20Type%20Object%20Reference) (InstigatedBy :type Controller%20Object%20Reference) (DamageCauser :type Actor%20Object%20Reference))
  (Variables|Default|SetHealth (- (Variables|Default|GetHealth) Damage))
  (if (<= (Variables|Default|GetHealth) 0.0)
    (Components|Activation|Deactivate (Variables|Character|GetCharacterMovement))
    (Animation|Montage|PlayMontage (Variables|Character|GetMesh) "/Game/Characters/FN_Husk/Animations/HuskMediumHitReactMontage.HuskMediumHitReactMontage"
      (:then
        (Effects|SpawnEmitteratLocation "/Game/Weapons/FORT_Pistols/Effects/P_Pistol_Impact_Med_SmokeOnly.P_Pistol_Impact_Med_SmokeOnly" (Transformation|GetActorLocation))
        (Utilities|FlowControl|Delay 0.6)
        (Actor|DestroyActor)))))

(fn ConstructionScript)